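; NPC guard AI controller that starts the GuardBehaviour tree with its blackboard and feeds it perception of player-tagged actors.
; A sensed stimulus tagged Hearing writes the player's current location to the last-seen-location key, while any other sensed stimulus sets the player as the enemy.
; An unsuccessful stimulus from the player, whatever its tag, clears the enemy key.
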(event `self.ReceiveBeginPlay`
  (bind _blackboardcomponent (`self.UseBlackboard` "/Game/NPC/AI/GuardBehaviourData.GuardBehaviourData"))
  (set `self.BlackboardComp` _blackboardcomponent)
  (`self.RunBehaviorTree` "/Game/NPC/AI/GuardBehaviour.GuardBehaviour"))

(event `self.AISightPerception.OnTargetPerceptionUpdated`
  (params (Actor :type "Actor Object Reference") (Stimulus :type "AIStimulus Structure"))
  (bind (_age _expirationage _strength _stimuluslocation _receiverlocation _tag _bsuccessfullysensed) (break `AIStimulus` Stimulus))
  (if (`KismetSystemLibrary.IsValid` Actor)
    (if (`self.ActorHasTag` Actor "Player")
      (if _bsuccessfullysensed
        (if (== _tag "Hearing")
          (`BlackboardComponent.SetValueAsVector` (`self.BlackboardComp`) (`self.LastSeenLocationKeyName`) (`self.K2_GetActorLocation` Actor))
          (else
            (`BlackboardComponent.SetValueAsObject` (`self.BlackboardComp`) (`self.EnemyKeyName`) Actor)))
        (else
          (`BlackboardComponent.ClearValue` (`self.BlackboardComp`) (`self.EnemyKeyName`)))))))

(fn `UserConstructionScript`)