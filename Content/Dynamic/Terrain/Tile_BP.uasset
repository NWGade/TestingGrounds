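; Terrain tile actor with a barrier that opens while the player overlaps the tile.
; It starts locked, and overlap events from actors tagged Player unlock it on entry and relock it on exit.
; Locking and unlocking toggle the barrier mesh's collision and swap its material between red and green.
; It also exposes the world transform of its AttachPoint component.
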(event `self.ReceiveBeginPlay`
  (`self.LockBarrier`))

(event `self.ReceiveActorEndOverlap`
  (params (OtherActor :type "Actor Object Reference"))
  (if (`self.ActorHasTag` OtherActor "Player")
    (`self.LockBarrier`)))

(event `self.ReceiveActorBeginOverlap`
  (params (OtherActor :type "Actor Object Reference"))
  (if (`self.ActorHasTag` OtherActor "Player")
    (`self.UnlockBarrier`)))

(fn `GetAttachPointTransform`
  (returns (AttachPointTransform :type "Transform Structure"))
  (return (`SceneComponent.K2_GetComponentToWorld` (`self.AttachPoint`))))

(fn `LockBarrier`
  (`PrimitiveComponent.SetCollisionEnabled` (`self.BarrierMesh`) "QueryAndPhysics")
  (`PrimitiveComponent.SetMaterial` (`self.BarrierMesh`) 0 "/Game/Static/Geometry/Meshes/RedBarrierMaterial.RedBarrierMaterial"))

(fn `UnlockBarrier`
  (`PrimitiveComponent.SetCollisionEnabled` (`self.BarrierMesh`) "NoCollision")
  (`PrimitiveComponent.SetMaterial` (`self.BarrierMesh`) 0 "/Game/Static/Geometry/Meshes/GreenBarrierMaterial.GreenBarrierMaterial"))

(fn `UserConstructionScript`)