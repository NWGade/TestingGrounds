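; AI controller for guard NPCs that runs the GuardBehaviour tree and reacts to perceived actors tagged Player.
; Stimuli tagged Hearing store the player's location as last seen, other successful stimuli set the player as enemy, and any lost stimulus clears the enemy.
; Each tick it sets the controlled ThirdPersonCharacter_BP's aiming and shooting flags according to whether the controller has a valid focus actor.
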(event `self.ReceiveBeginPlay`
  (bind _blackboardcomponent (`self.UseBlackboard` "/Game/Dynamic/NPC/AI/GuardBehaviourData.GuardBehaviourData"))
  (set `self.BlackboardComp` _blackboardcomponent)
  (`self.RunBehaviorTree` "/Game/Dynamic/NPC/AI/GuardBehaviour.GuardBehaviour"))

(event `self.ReceiveTick`
  (params (DeltaSeconds :type "Float (single-precision)"))
  (bind _returnvalue (`KismetSystemLibrary.IsValid` (`self.GetFocusActor`)))
  (bind _asthird_person_character_bp (cast `/Game/Dynamic/NPC/Blueprints/ThirdPersonCharacter_BP` (`self.K2_GetPawn`)))
  (set `/Game/Dynamic/NPC/Blueprints/ThirdPersonCharacter_BP.AIming` _returnvalue _asthird_person_character_bp)
  (set `/Game/Dynamic/NPC/Blueprints/ThirdPersonCharacter_BP.Shooting` _returnvalue _asthird_person_character_bp))

(event `self.AISightPerception.OnTargetPerceptionUpdated`
  (params (Actor :type "Actor Object Reference") (Stimulus :type "AIStimulus Structure"))
  (bind (_age _expirationage _strength _stimuluslocation _receiverlocation _tag _bsuccessfullysensed) (break `AIStimulus` Stimulus))
  (if (`KismetSystemLibrary.IsValid` Actor)
    (if (`self.ActorHasTag` Actor "Player")
      (if _bsuccessfullysensed
        (if (== _tag "Hearing")
          (`BlackboardComponent.SetValueAsVector` (`self.BlackboardComp`) (`self.LastSeenLocationKeyName`) (`self.K2_GetActorLocation` Actor))
          (else
            (`BlackboardComponent.SetValueAsObject` (`self.BlackboardComp`) (`self.EnemyKeyName`) Actor)))
        (else
          (`BlackboardComponent.ClearValue` (`self.BlackboardComp`) (`self.EnemyKeyName`)))))))

(fn `UserConstructionScript`)